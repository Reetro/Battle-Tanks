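; Player-controllable tank Blueprint that hands movement, aiming and firing to dedicated components.
; On BeginPlay it passes the barrel and turret to TankAiming, and the left and right tracks to TankMovement.
; Axis inputs send forward and turn intents to TankMovement, while the Fire action calls TankAiming.
; Camera aim yaws an azimuth gimbal and pitches the spring arm separately, with rotation scaled by frame delta time.
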(event `self.ReceiveBeginPlay`
  (`TankAimingComponent.Initialize` (`self.TankAiming`) (`self.Barrrel`) (`self.Turret`))
  (`TankMovementComponent.Initialize` (`self.TankMovement`) (`self.Left Track`) (`self.Right Track`)))

(event `InputAxis|MoveFoward`
  (params (AxisValue :type "Float (single-precision)"))
  ;[1 1 1] Movement Inputs
  (`TankMovementComponent.IntendMoveForward` (`self.TankMovement`) AxisValue))

(event `InputAxis|AimAzimuth`
  (params (AxisValue :type "Float (single-precision)"))
  ;[1 1 1] Camera Input Binding
  ;;[0 0 0] Move Camera Left and Right
  (`SceneComponent.K2_AddLocalRotation` (`self.Azimuth Gimble`) (`KismetMathLibrary.MakeRotator` 0.0 0.0 (* AxisValue (`GameplayStatics.GetWorldDeltaSeconds`) 100.0)) false false))

(event `InputAxis|TurnRight`
  (params (AxisValue :type "Float (single-precision)"))
  ;[1 1 1] Movement Inputs
  (`TankMovementComponent.IntendTurn` (`self.TankMovement`) AxisValue))

(event `InputAxis|AimElevation`
  (params (AxisValue :type "Float (single-precision)"))
  ;[1 1 1] Camera Input Binding
  ;;[0 0 0] Move Camera Up and Down
  (`SceneComponent.K2_AddLocalRotation` (`self.SpringArm`) (`KismetMathLibrary.MakeRotator` 0.0 (* AxisValue (`GameplayStatics.GetWorldDeltaSeconds`) 100.0)) false false))

(event `InputAction|Fire`
  (params (Key :type "Key Structure"))
  ;[1 1 1] Fire Gun
  (:`Pressed`
    (`TankAimingComponent.FireGun` (`self.TankAiming`))))

(fn `UserConstructionScript`)